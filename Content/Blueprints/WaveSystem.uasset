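; Wave spawner that releases BasicEnemy creeps at random CreepSpawns points and sends them toward a shared Goal.
; StartWave arms a wave once no creeps remain; Tick spawns them at random intervals while unpaused.
; DeductCreep lowers the alive count that IsWaveOver checks.
; WaveIncreaseFactor growth applies only when CurrentWaveSize differs from InitialWaveSize, which nothing here causes after construction equalises them, so waves stay the same size.
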(event EventBeginPlay)

(event Collision|EventActorBeginOverlap
  (params (OtherActor :type Actor%20Object%20Reference)))

(event EventTick
  (params (DeltaSeconds :type Float%20%28single-precision%29))
  (if (> (Variables|Default|GetToSpawnWaveSize) 0)
    (if (not (Game|IsGamePaused))
      (Variables|Default|SetTimeToNextSpawn (- (Variables|Default|GetTimeToNextSpawn) DeltaSeconds))
      (if (<= (Variables|Default|GetTimeToNextSpawn) 0.0)
        (CallFunction|SpawnCreep)))))

(fn ConstructionScript
  (Variables|Default|SetCurrentWaveSize (Variables|Default|GetInitialWaveSize)))

(fn StartWave
  ;[1 1 1] See If any creeps are left from last wave
  (if (<= (Variables|Default|GetCreepsAlive) 0)
    (if (== (Variables|Default|GetCurrentWaveSize) (Variables|Default|GetInitialWaveSize))
      ;[1 1 1] Set How Many Creeps Will Spawn, Are Allive, & time to first spawn
      (bind _output_get (Variables|Default|SetToSpawnWaveSize (Variables|Default|GetCurrentWaveSize)))
      (Variables|Default|SetCreepsAlive _output_get)
      (Variables|Default|SetTimeToNextSpawn (Math|Random|RandomFloatinRange (Variables|Default|GetTimeBetweenSpawns_Min) (Variables|Default|GetTimeBetweenSpawns_Max)))
      (else
        ;[1 1 1] If not calculate how many creeps will be spawned this wave
        (bind _output_get_2 (Variables|Default|SetCurrentWaveSize (+ (Variables|Default|GetCurrentWaveSize) (Math|Float|Truncate (* (Variables|Default|GetCurrentWaveSize) (Variables|Default|GetWaveIncreaseFactor))))))
        ;[1 1 1] Set How Many Creeps Will Spawn, Are Allive, & time to first spawn
        (bind _output_get_3 (Variables|Default|SetToSpawnWaveSize _output_get_2))
        (Variables|Default|SetCreepsAlive _output_get_3)
        (Variables|Default|SetTimeToNextSpawn (Math|Random|RandomFloatinRange (Variables|Default|GetTimeBetweenSpawns_Min) (Variables|Default|GetTimeBetweenSpawns_Max)))))))

(fn IsWaveOver
  (return (<= (Variables|Default|GetCreepsAlive) 0)))

(fn DeductCreep
  (Math|Integer|DecrementInt (Variables|Default|GetCreepsAlive)))

(fn SpawnCreep
  (bind _creepspawns (Variables|Default|GetCreepSpawns))
  (bind _returnvalue (Game|SpawnActorfromClass "/Game/TowerDefense/Blueprints/Enemies/BasicEnemy.BasicEnemy_C" (Transformation|GetActorTransform (Utilities|Array|Get(acopy) _creepspawns (Math|Random|RandomIntegerinRange 0 (- (Utilities|Array|Length _creepspawns) 1)))) "AdjustIfPossibleButDontSpawnIfColliding" 0 0))
  (Variables|/Game/TowerDefense/Blueprints/Enemies/BasicEnemy.BasicEnemy_C|SetGoal _returnvalue (Variables|Default|GetGoal))
  (Default|InitializeEnemy _returnvalue)
  (Variables|Default|SetTimeToNextSpawn (Math|Random|RandomFloatinRange (Variables|Default|GetTimeBetweenSpawns_Min) (Variables|Default|GetTimeBetweenSpawns_Max)))
  (Math|Integer|DecrementInt (Variables|Default|GetToSpawnWaveSize)))