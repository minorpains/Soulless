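; ArcherTwer is an archer tower Blueprint for a tower defense game that turns its cannon to face enemies.
; Each tick its BasicTwrTargetingComponent checks for targets, and when any are found the Cannon yaws toward the first enemy in the temporary array, keeping its pitch and roll.
; Attack and the construction script only call their parent versions, so no attack logic is defined here.
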(event EventBeginPlay)

(event EventTick
  (params (DeltaSeconds :type Float%20%28single-precision%29))
  (bind _basictwrtargetingcomponent (Variables|Default|GetBasicTwrTargetingComponent))
  (bind _cannon (Variables|Default|GetCannon))
  (bind _returnvalue (Transformation|GetWorldRotation _cannon))
  (bind _temporaryenemiesarray (Variables|/Game/TowerDefense/Blueprints/Components/TargetingComponents/BasicTwrTargetingComponent.BasicTwrTargetingComponent_C|GetTemporaryEnemiesArray _basictwrtargetingcomponent))
  (bind (_roll _pitch) (Math|Rotator|BreakRotator _returnvalue))
  (Utilities|IsValid 0
    (:Is%20Valid
      _)
    (:Is%20Not%20Valid
      _))
  (Default|CheckforTarget (Variables|Default|GetBasicTwrTargetingComponent))
  (if (>= (Utilities|Array|Length _temporaryenemiesarray) 1)
    (Transformation|SetWorldRotation _cannon (Math|Rotator|MakeRotator _roll _pitch (.Yaw (Math|Rotator|BreakRotator (Math|Rotator|FindLookatRotation (Transformation|GetWorldLocation (Variables|Default|GetCannon)) (Transformation|GetActorLocation (Utilities|Array|Get(acopy) _temporaryenemiesarray)))))) false false)))

(fn ConstructionScript
  (|CallParentFunction))

(fn Attack
  (|CallParentFunction)
  (return))