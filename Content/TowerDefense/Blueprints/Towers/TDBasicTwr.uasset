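; TDBasicTwr is a tower actor for the tower defense game that delegates its attack to separate targeting and weapon components.
; On BeginPlay it records the FakeOrigin world location, then caches its targeting and weapon components, printing an error if either is missing or duplicated.
; Attack passes the result of the targeting component's CheckForTarget to the weapon component's Fire, printing an error if either reference is invalid.
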(event EventBeginPlay
  (bind _returnvalue (Actor|GetComponentsByClass "/Game/TowerDefense/Blueprints/Components/WeaponComponents/BasicTwrWeaponComponent.BasicTwrWeaponComponent_C"))
  (bind _returnvalue_2 (Actor|GetComponentsByClass "/Game/TowerDefense/Blueprints/Components/TargetingComponents/BasicTwrTargetingComponent.BasicTwrTargetingComponent_C"))
  (bind _returnvalue_3 (Utilities|Array|Length _returnvalue))
  (bind _returnvalue_4 (Utilities|Array|Length _returnvalue_2))
  (Variables|Default|SetFakeOriginLocation (Transformation|GetWorldLocation (Variables|Default|GetFakeOrigin)))
  (if (> _returnvalue_4 1)
    (Development|PrintString "A tower has multiple targeting elements. PLease remove one or more." true true "(R=0.450000,G=0.027189,B=0.054066,A=1.000000)")
    (elif (<= _returnvalue_4 0)
      (Development|PrintString "A tower has no targeting component. Please add one." true true "(R=0.450000,G=0.438498,B=0.020691,A=1.000000)")
      (else
        (Variables|Default|SetTwrTargetingComponent (Utilities|Array|Get(acopy) _returnvalue_2))
        (if (> _returnvalue_3 1)
          (Development|PrintString "A tower has multiple weapon elements. PLease remove one or more." true true "(R=0.450000,G=0.027189,B=0.054066,A=1.000000)")
          (elif (<= _returnvalue_3 0)
            (Development|PrintString "A tower has no weapon component. Please add one." true true "(R=0.450000,G=0.027189,B=0.054066,A=1.000000)")
            (else
              (Variables|Default|SetTwrWeaponComponent (Utilities|Array|Get(acopy) _returnvalue)))))))))

(fn ConstructionScript)

(fn Attack
  (bind _twrtargetingcomponent (Variables|Default|GetTwrTargetingComponent))
  (bind _twrweaponcomponent (Variables|Default|GetTwrWeaponComponent))
  (Utilities|IsValid _twrtargetingcomponent
    (:Is%20Valid
      (bind _enemiesfound (Default|CheckforTarget _twrtargetingcomponent))
      (Utilities|IsValid _twrweaponcomponent
        (:Is%20Valid
          (Default|Fire _twrweaponcomponent _enemiesfound))
        (:Is%20Not%20Valid
          (Development|PrintString "Tower Weapon Component is not valid"))))
    (:Is%20Not%20Valid
      (Development|PrintString "Tower Targeting Component is not valid"))))