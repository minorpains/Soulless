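; Basic tower defense enemy that loses health through ReceiveDamage and calls KillEnemy when health reaches zero.
; KillEnemy awards resources through TDGameMode, destroys the actor and plays a death cue.
; ReachBase removes the enemy without reward or base damage.
; Both exits hide the actor, switch capsule and mesh collision to the Vehicle object type, and deduct a creep from the first WaveSystem found.
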(event Custom|InitializeEnemy
  (AI|GetAIController self))

(event Collision|EventActorBeginOverlap
  (params (OtherActor :type Actor%20Object%20Reference)))

(event EventTick
  (params (DeltaSeconds :type Float%20%28single-precision%29)))

(fn ConstructionScript)

(fn ReceiveDamage
  (params (DamageAmt :type Integer))
  (bind _output_get (Variables|Default|SetHealth (- (Variables|Default|GetHealth) DamageAmt)))
  (if (<= _output_get 0)
    (CallFunction|KillEnemy)))

(fn KillEnemy
  (Rendering|SetActorHiddenInGame true)
  (Collision|SetCollisionObjectType (Variables|Default|GetCapsuleComponent) "ECC_Vehicle")
  (Collision|SetCollisionObjectType (Variables|Character|GetMesh) "ECC_Vehicle")
  (bind _astdgame_mode (Utilities|Casting|CastToTDGameMode (Game|GetGameMode)))
  (Default|AIGiveResurcesCallback _astdgame_mode (Variables|Default|GetResourceValueOnKilled) (Variables|Default|GetResourceTypeWhenKilled))
  (Actor|DestroyActor)
  (Audio|PlaySound2D "/Game/SFX/deathCue.deathCue")
  (bind _outactors (Actor|GetAllActorsOfClass "/Game/Blueprints/WaveSystem.WaveSystem_C"))
  (Default|DeductCreep (Utilities|Array|Get(acopy) _outactors)))

(fn ReachBase
  (Rendering|SetActorHiddenInGame true)
  (Collision|SetCollisionObjectType (Variables|Default|GetCapsuleComponent) "ECC_Vehicle")
  (Collision|SetCollisionObjectType (Variables|Character|GetMesh) "ECC_Vehicle")
  (Utilities|Casting|CastToTDGameMode (Game|GetGameMode))
  (Actor|DestroyActor)
  (bind _outactors (Actor|GetAllActorsOfClass "/Game/Blueprints/WaveSystem.WaveSystem_C"))
  (Default|DeductCreep (Utilities|Array|Get(acopy) _outactors)))