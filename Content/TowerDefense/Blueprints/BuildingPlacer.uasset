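; BuildingPlacer is the tower defense placement preview actor that shows whether a building can be placed at its current spot.
; Every Tick it checks for overlapping actors and calls SetCannotPlace if any exist, otherwise SetCanPlace.
; Those events swap the static mesh's first ten material slots to a translucent okay or error material and set the CanPlaceCurrently flag to match.
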(event Custom|SetCannotPlace
  ;[1 1 1] Set Material Instance for Placement Color
  (Rendering|Material|SetMaterial (Variables|Default|GetStaticMesh) 0 "/Game/TowerDefense/Materials/TowerTranslucentError.TowerTranslucentError")
  (Rendering|Material|SetMaterial (Variables|Default|GetStaticMesh) 1 "/Game/TowerDefense/Materials/TowerTranslucentError.TowerTranslucentError")
  (Rendering|Material|SetMaterial (Variables|Default|GetStaticMesh) 2 "/Game/TowerDefense/Materials/TowerTranslucentError.TowerTranslucentError")
  (Rendering|Material|SetMaterial (Variables|Default|GetStaticMesh) 3 "/Game/TowerDefense/Materials/TowerTranslucentError.TowerTranslucentError")
  (Rendering|Material|SetMaterial (Variables|Default|GetStaticMesh) 4 "/Game/TowerDefense/Materials/TowerTranslucentError.TowerTranslucentError")
  (Rendering|Material|SetMaterial (Variables|Default|GetStaticMesh) 5 "/Game/TowerDefense/Materials/TowerTranslucentError.TowerTranslucentError")
  (Rendering|Material|SetMaterial (Variables|Default|GetStaticMesh) 6 "/Game/TowerDefense/Materials/TowerTranslucentError.TowerTranslucentError")
  (Rendering|Material|SetMaterial (Variables|Default|GetStaticMesh) 7 "/Game/TowerDefense/Materials/TowerTranslucentError.TowerTranslucentError")
  (Rendering|Material|SetMaterial (Variables|Default|GetStaticMesh) 8 "/Game/TowerDefense/Materials/TowerTranslucentError.TowerTranslucentError")
  (Rendering|Material|SetMaterial (Variables|Default|GetStaticMesh) 9 "/Game/TowerDefense/Materials/TowerTranslucentError.TowerTranslucentError")
  (Variables|Default|SetCanPlaceCurrently false))

(event Custom|SetCanPlace
  ;[1 1 1] Set Material Instance for Placement Color
  (Rendering|Material|SetMaterial (Variables|Default|GetStaticMesh) 0 "/Game/TowerDefense/Materials/TowerTranslucentOkay.TowerTranslucentOkay")
  (Rendering|Material|SetMaterial (Variables|Default|GetStaticMesh) 1 "/Game/TowerDefense/Materials/TowerTranslucentOkay.TowerTranslucentOkay")
  (Rendering|Material|SetMaterial (Variables|Default|GetStaticMesh) 2 "/Game/TowerDefense/Materials/TowerTranslucentOkay.TowerTranslucentOkay")
  (Rendering|Material|SetMaterial (Variables|Default|GetStaticMesh) 3 "/Game/TowerDefense/Materials/TowerTranslucentOkay.TowerTranslucentOkay")
  (Rendering|Material|SetMaterial (Variables|Default|GetStaticMesh) 4 "/Game/TowerDefense/Materials/TowerTranslucentOkay.TowerTranslucentOkay")
  (Rendering|Material|SetMaterial (Variables|Default|GetStaticMesh) 5 "/Game/TowerDefense/Materials/TowerTranslucentOkay.TowerTranslucentOkay")
  (Rendering|Material|SetMaterial (Variables|Default|GetStaticMesh) 6 "/Game/TowerDefense/Materials/TowerTranslucentOkay.TowerTranslucentOkay")
  (Rendering|Material|SetMaterial (Variables|Default|GetStaticMesh) 7 "/Game/TowerDefense/Materials/TowerTranslucentOkay.TowerTranslucentOkay")
  (Rendering|Material|SetMaterial (Variables|Default|GetStaticMesh) 8 "/Game/TowerDefense/Materials/TowerTranslucentOkay.TowerTranslucentOkay")
  (Rendering|Material|SetMaterial (Variables|Default|GetStaticMesh) 9 "/Game/TowerDefense/Materials/TowerTranslucentOkay.TowerTranslucentOkay")
  (Variables|Default|SetCanPlaceCurrently true))

(event EventBeginPlay)

(event EventTick
  (params (DeltaSeconds :type Float%20%28single-precision%29))
  (if (> (Utilities|Array|Length (Collision|GetOverlappingActors 0 :!class /Script/Engine.Actor)) 0)
    (CallFunction|SetCannotPlace)
    (else
      (CallFunction|SetCanPlace))))

(fn ConstructionScript)