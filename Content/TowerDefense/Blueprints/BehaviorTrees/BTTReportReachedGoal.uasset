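; Behavior tree task that reports a BasicEnemy reaching its goal in the tower defense game.
; It passes the AI controller's pawn to TDGameMode's AIGoalReachedCallback, then finishes successfully.
; A gate closes after each report and a timer reopens it seconds later, throttling repeat calls.
; Finish is only called on a successful report, so blocked or failed-cast executions leave the task unfinished.
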(event Custom|CloseGate
  (Utilities|FlowControl|Gate false) ; enters at Close
)

(event Custom|OpenGate
  (Utilities|FlowControl|Gate false) ; enters at Open
)

(event EventReceiveExecute
  (params (OwnerActor :type Actor%20Object%20Reference))
  (Utilities|FlowControl|Gate false
    (:Exit
      (bind _asaicontroller (Utilities|Casting|CastToAIController OwnerActor)
        (:then
          (bind _asbasic_enemy (Utilities|Casting|CastToBasicEnemy (Pawn|GetControlledPawn _asaicontroller))
            (:then
              (bind _astdgame_mode (Utilities|Casting|CastToTDGameMode (Game|GetGameMode)))
              (Default|AIGoalReachedCallback _astdgame_mode _asbasic_enemy)
              (CallFunction|CloseGate)
              (Utilities|Time|SetTimerbyFunctionName 0 "OpenGate" 3.0)
              (AI|BehaviorTree|FinishExecute true))
            (:CastFailed
              (Development|PrintString "BTTReachedReport Failed a cast" true true "(R=1.000000,G=0.000000,B=0.000000,A=1.000000)" :!label _label))))
        (:CastFailed
          (goto _label))))))