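; Tower defense game mode that tracks base health, resources and score, and caches the level's goals and spawn points at BeginPlay.
; Enemies reaching a goal subtract their damage from player health; at zero, it shows the main menu and restarts the level.
; Callbacks add gold, stone, wood, metal or score, but deduction only affects gold, ignoring the resource type passed in.
; Helpers expose health percentage and gold affordability checks.
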(event EventBeginPlay
  (bind _outactors (Actor|GetAllActorsOfClass "/Game/TowerDefense/Blueprints/Goal.Goal_C"))
  (Variables|Default|SetEnemyGoals _outactors)
  (bind _outactors_2 (Actor|GetAllActorsOfClass "/Game/TowerDefense/Blueprints/SpawnPoint.SpawnPoint_C"))
  (Variables|Default|SetSpawnPoints _outactors_2)
  (Variables|Default|SetCurrentPlayerHealth (Variables|Default|GetStartingPlayerHealth)))

(event EventTick
  (params (DeltaSeconds :type Float%20%28single-precision%29)))

(fn ConstructionScript)

(fn AIGoalReachedCallback
  (params (ControlledEnemy :type Basic%20Enemy%20Object%20Reference))
  (bind _output_get (Variables|Default|SetCurrentPlayerHealth (- (Variables|Default|GetCurrentPlayerHealth) (Variables|/Game/TowerDefense/Blueprints/Enemies/BasicEnemy.BasicEnemy_C|GetDamageOnReachingGoal ControlledEnemy))))
  (Default|ReachBase ControlledEnemy)
  (Audio|PlaySound2D "/Game/SFX/baseDamage.baseDamage")
  (if (<= _output_get 0)
    (CallFunction|DoPlayerDeath)))

(fn DoPlayerDeath
  (Viewport|RemoveAllWidgets)
  (bind _returnvalue (UserInterface|CreateWidget "/Game/UI/MainMenu.MainMenu_C"))
  (UserInterface|Viewport|AddtoViewport _returnvalue 0)
  (Variables|/Script/Engine.PlayerController|SetbShowMouseCursor (Game|GetPlayerController 0) true)
  (Development|ExecuteConsoleCommand "RestartLevel"))

(fn GetPlayerHealthPercent
  (return (/ (Math|Conversions|ToFloat(Integer) (Variables|Default|GetCurrentPlayerHealth)) (Math|Conversions|ToFloat(Integer) (Variables|Default|GetStartingPlayerHealth)))))

(fn AIGiveResurcesCallback
  (params (ResourceAmount :type Integer) (ResourceType :type ResourceTypeEnums%20Enum))
  (switch Utilities|FlowControl|Switch|SwitchonResourceTypeEnums ResourceType
    (:NewEnumerator0
      (Variables|Default|SetCurrentPlayerGold (+ (Variables|Default|GetCurrentPlayerGold) ResourceAmount)))
    (:NewEnumerator1
      (Variables|Default|SetCurrentPlayerStone (+ (Variables|Default|GetCurrentPlayerStone) ResourceAmount)))
    (:NewEnumerator2
      (Variables|Default|SetCurrentPlayerWood (+ (Variables|Default|GetCurrentPlayerWood) ResourceAmount)))
    (:NewEnumerator3
      (Variables|Default|SetCurrentPlayerMetal (+ (Variables|Default|GetCurrentPlayerMetal) ResourceAmount)))
    (:NewEnumerator4
      (Variables|Default|SetCurrentPlayerScore (+ (Variables|Default|GetCurrentPlayerScore) ResourceAmount)))))

(fn AITakeResourcesCallback
  (params (Resource%20Amount :type Integer) (Resource%20Type :type ResourceTypeEnums%20Enum))
  (switch Utilities|FlowControl|Switch|SwitchonResourceTypeEnums "NewEnumerator0"
    (:NewEnumerator0
      (Variables|Default|SetCurrentPlayerGold (- (Variables|Default|GetCurrentPlayerGold) Resource%20Amount)))))

(fn GoldCheck
  (params (Cost :type Integer))
  (bind _currentplayergold (Variables|Default|GetCurrentPlayerGold))
  (bind _returnvalue (<= Cost _currentplayergold))
  (if _returnvalue
    (return _returnvalue)
    (else
      (return false))))