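; BasicBullet is a tower defense projectile that flies straight and damages the enemy it hits.
; Each tick it moves its Sphere component along that component's forward vector at ProjectileSpeed scaled by delta time, using a swept teleport transform update.
; On overlapping a BasicEnemy it passes Damage to that enemy's ReceiveDamage and destroys itself, ignoring other actors.
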(event EventBeginPlay)

(event Collision|EventActorBeginOverlap
  (params (OtherActor :type Actor%20Object%20Reference))
  (bind _asbasic_enemy (Utilities|Casting|CastToBasicEnemy OtherActor))
  (Default|ReceiveDamage _asbasic_enemy (Variables|Default|GetDamage))
  (Actor|DestroyActor))

(event EventTick
  (params (DeltaSeconds :type Float%20%28single-precision%29))
  (bind _sphere (Variables|Default|GetSphere))
  (bind _returnvalue (Transformation|GetWorldTransform _sphere))
  (bind (_location _rotation _scale) (Math|Transform|BreakTransform _returnvalue))
  (Transformation|SetWorldTransform (Variables|Default|GetSphere) (Math|Transform|MakeTransform (+ _location (* (Math|Vector|GetForwardVector _rotation) (* (Variables|Default|GetProjectileSpeed) (Utilities|Time|GetWorldDeltaSeconds)))) _rotation _scale) true true))

(fn ConstructionScript)