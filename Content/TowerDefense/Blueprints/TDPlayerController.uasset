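; Tower defense player controller that creates the resource and tower placement UI, moves the pawn, and handles tower placement.
; Placement mode spawns the tower out of view and copies its mesh to a BuildingPlacer preview.
; Each tick, a cursor trace snaps the preview to a 100-unit grid, or parks it high above when inactive.
; Confirm moves the tower there if placement is allowed, while Cancel destroys any pending tower and exits.
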(event Custom|StartTowerPlacementMode
  (params (TowerClassToCreate :type TD%20Basic%20Twr%20Class%20Reference))
  ;[1 1 1] Building Placement Functions
  (Variables|Default|SetIsInBuildingPlaceMode true)
  (bind _returnvalue (Game|SpawnActorfromClass TowerClassToCreate (Math|Transform|MakeTransform "0, 0,10000.000000") "AlwaysSpawn" 0 0))
  (bind _output_get (Variables|Default|SetTowerReadyToConstruct _returnvalue))
  (Components|StaticMesh|SetStaticMesh (Variables|/Game/TowerDefense/Blueprints/BuildingPlacer.BuildingPlacer_C|GetStaticMesh (Variables|Default|GetBuildingPlacer)) (Variables|/Script/Engine.StaticMeshComponent|GetStaticMesh (Variables|/Game/TowerDefense/Blueprints/Towers/TDBasicTwr.TDBasicTwr_C|GetBasicTwr _output_get))))

(event Custom|EndTowerPlacementMode
  (bind _towerreadytoconstruct (Variables|Default|GetTowerReadyToConstruct))
  ;[1 1 1] Building Placement Functions
  (Variables|Default|SetIsInBuildingPlaceMode false)
  (Utilities|IsValid _towerreadytoconstruct
    (:Is%20Valid
      (Actor|DestroyActor _towerreadytoconstruct))))

(event Custom|PlaceTower
  (bind _buildingplacer (Variables|Default|GetBuildingPlacer))
  ;[1 1 1] Building Placement Functions
  (if (Variables|/Game/TowerDefense/Blueprints/BuildingPlacer.BuildingPlacer_C|GetCanPlaceCurrently _buildingplacer)
    (Transformation|SetActorLocation (Variables|Default|GetTowerReadyToConstruct) (Transformation|GetActorLocation _buildingplacer) false true)
    (Variables|Default|SetTowerReadyToConstruct 0)))

(event EventBeginPlay
  ;[1 1 1] Comment
  (bind _astddefault_player_pawn (Utilities|Casting|CastToTDDefaultPLayerPawn (Pawn|GetControlledPawn))
    (:then
      (Variables|Default|SetPlayerPawn _astddefault_player_pawn)
      (bind _returnvalue (UserInterface|CreateWidget "/Game/TowerDefense/Blueprints/UI/PlayerResourcesPanel.PlayerResourcesPanel_C"))
      (UserInterface|Viewport|AddtoViewport _returnvalue 0)
      (bind _returnvalue_2 (UserInterface|CreateWidget "/Game/TowerDefense/Blueprints/UI/TowerPlacementPanel.TowerPlacementPanel_C"))
      (UserInterface|Viewport|AddtoViewport _returnvalue_2 0)
      (bind _returnvalue_3 (Game|SpawnActorfromClass "/Game/TowerDefense/Blueprints/BuildingPlacer.BuildingPlacer_C" (Math|Transform|MakeTransform "0, 0,10000.000000") "AlwaysSpawn" 0 0))
      (Variables|Default|SetBuildingPlacer _returnvalue_3))
    (:CastFailed
      (Development|PrintString "TD Player Controller could not cast to to TDplayerPawn" true true "(R=0.305000,G=0.021535,B=0.000000,A=1.000000)"))))

(event EventTick
  (params (DeltaSeconds :type Float%20%28single-precision%29))
  (bind _array (Utilities|Array|MakeArray "ObjectTypeQuery9"))
  (bind _hitresult (Class|PlayerController|GetHitResultUnderCursorforObjects _array true))
  (bind _location (Collision|BreakHitResult _hitresult))
  (bind (_x _y) (Math|Vector|BreakVector _location))
  (if (Variables|Default|GetIsInBuildingPlaceMode)
    (Transformation|SetActorLocation (Variables|Default|GetBuildingPlacer) (Math|Vector|MakeVector (* (.ReturnValue (Math|Float|Division(WholeandRemainder) (+ _x 1e+02) 1e+02)) 1e+02) (* (.ReturnValue (Math|Float|Division(WholeandRemainder) (+ _y 1e+02) 1e+02)) 1e+02) 0.0) false true)
    (else
      (Transformation|SetActorLocation (Variables|Default|GetBuildingPlacer) "0, 0,10000.000000" false true))))

(event Input|ActionEvents|InputActionCancel
  (params (Key :type Key%20Structure :default "AnyKey"))
  ;[1 1 1] Cancel
  (:Pressed
    (if (Variables|Default|GetIsInBuildingPlaceMode)
      (CallFunction|EndTowerPlacementMode))))

(event Input|ActionEvents|InputActionConfirm
  (params (Key :type Key%20Structure :default "AnyKey"))
  ;[1 1 1] Confirm
  (:Pressed
    (if (Variables|Default|GetIsInBuildingPlaceMode)
      (CallFunction|PlaceTower))))

(event Input|AxisEvents|InputAxisMovesRight
  (params (AxisValue :type Float%20%28single-precision%29))
  ;[1 1 1] Horizontal Movement
  (Pawn|Input|AddMovementInput (Variables|Default|GetPlayerPawn) "1.000000, 0, 0" AxisValue false))

(event Input|AxisEvents|InputAxisMoveUp
  (params (AxisValue :type Float%20%28single-precision%29))
  ;[1 1 1] Vertical Movement
  (Pawn|Input|AddMovementInput (Variables|Default|GetPlayerPawn) "0.000000,-1.000000, 0" AxisValue false))

(fn ConstructionScript)